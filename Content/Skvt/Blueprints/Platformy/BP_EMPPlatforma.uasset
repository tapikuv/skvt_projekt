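; EMP platform Blueprint that sets off an area EMP when something overlaps its Box.
; The overlap runs a relevant-actor search within a fixed radius around the box, feeding results to Rozmlat.
; Rozmlat calls AplikujEMP on results through the BPI_EMP interface.
; The local NajdiRelevantniAktory function, whose signature differs from that call, sphere-overlaps, applies EMP itself, draws a debug sphere and prints affected names.
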(event OnComponentBeginOverlap(Box)
  (params (OverlappedComponent :type Primitive%20Component%20Object%20Reference) (OtherActor :type Actor%20Object%20Reference) (OtherComp :type Primitive%20Component%20Object%20Reference) (OtherBodyIndex :type Integer) (bFromSweep :type Boolean) (SweepResult :type Hit%20Result%20Structure%20%28by%20ref%29))
  (bind _empik (Utilities|NajdiRelevantniAktory (Transformation|GetWorldLocation OverlappedComponent) 5e+02 (Variables|Default|GetObject%20Types) (Variables|Default|GetDebug))
    (:forEachDo
      (Utilities|Rozmlat _empik))))

(event EventBeginPlay)

(event EventTick
  (params (DeltaSeconds :type Float%20%28single-precision%29)))

(fn ConstructionScript)

(fn Rozmlat
  (params (Empici :type Array%20of%20Actor%20Object%20References))
  (for _array_element Empici
    (bind _asbpi_emp (Utilities|Casting|CastToBPI_EMP _array_element))
    (Default|AplikujEMP _asbpi_emp)))

(fn NajdiRelevantniAktory
  (params (Poloha :type Vector))
  (bind _outactors (Collision|SphereOverlapActors Poloha 5e+02 (Variables|Default|GetObject%20Types) 0))
  (Rendering|Debug|DrawDebugSphere Poloha 5e+02 12 "(R=1.000000,G=1.000000,B=1.000000,A=1.000000)" 1e+01 2.0)
  (for _array_element _outactors
    (bind _asbpi_emp (Utilities|Casting|CastToBPI_EMP _array_element))
    (Default|AplikujEMP _asbpi_emp)
    (Development|PrintString (Utilities|GetObjectName (Utilities|ToObject(Interface) _asbpi_emp))))
  (return 0 0))