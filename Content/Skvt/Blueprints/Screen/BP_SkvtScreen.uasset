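; BP_SkvtScreen is an in-world screen showing a web page through a widget component, with switch-off and EMP reactions.
; On BeginPlay it caches the WBP_SkvtWeb widget and marks itself on.
; Vypnout (turn off) hides the component unless broken; AplikujEMP breaks a powered, intact screen and redirects its browser to Bing.
; Other cases only print Czech messages, and Rozsvit (light up) is an empty stub.
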(event EventBeginPlay
  (CallFunction|Initialize))

(event Collision|EventActorBeginOverlap
  (params (OtherActor :type Actor%20Object%20Reference)))

(event EventTick
  (params (DeltaSeconds :type Float%20%28single-precision%29)))

(event EventVypnout
  (if (Variables|Default|GetJeRozbitej)
    (Development|PrintText "Je Rozbitej")
    (else
      (CallFunction|Toggleon self false))))

(event EventAplikujEMP
  (if (Variables|Default|GetJeRozbitej)
    (Development|PrintText "Pozdrav ze zahrobi")
    (elif (Variables|Default|GetIsOn)
      (Variables|Default|SetJeRozbitej true)
      (Class|WebBrowser|LoadURL (Variables|/Game/Skvt/Blueprints/Screen/WBP_SkvtWeb.WBP_SkvtWeb_C|GetSkvtBrowser (Variables|Default|GetWebpageRef)) "https://www.bing.com")
      (else
        (Development|PrintText "Jsem v jinem vesmiru, smula")))))

(event EventRozsvit
  (params (MaSvitit :type Boolean)))

(fn ConstructionScript)

(fn Initialize
  (bind _aswbp_skvt_web (Utilities|Casting|CastToWBP_SkvtWeb (UserInterface|GetWidget (Variables|Default|GetWebpage))))
  (Variables|Default|SetWebpageRef _aswbp_skvt_web)
  (Variables|Default|SetIsOn true))

(fn Toggleon
  (params (TurnOn :type Boolean))
  (Rendering|SetVisibility (Variables|Default|GetWebpage) TurnOn false)
  (Variables|Default|SetIsOn TurnOn))