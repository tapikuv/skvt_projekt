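; BP_WallSconce is a wall sconce light with a cone light (SconceLight) and a bulb light (Zarovicka).
; Construction applies shared brightness, cone angles and color, gives the bulb a fixed warm tint, and shows SconceLight according to Svitime.
; NastavRoznuti sets that state and toggles only SconceLight; the Vypnout event uses it to switch off.
; Zruď forces SconceLight visible and intense red without updating Svitime.
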(event EventVypnout
  (CallFunction|NastavRoznuti self false))

(fn ConstructionScript
  (CallFunction|OriginalniInicializaceLampy)
  (Rendering|SetVisibility (Variables|Default|GetSconceLight) (Variables|Moje|GetSvitime) false))

(fn OriginalniInicializaceLampy
  (bind _sconcelight (Variables|Default|GetSconceLight))
  (Rendering|Components|Light|SetIntensity (Variables|Default|GetZarovicka) (Variables|Light|GetBrightness))
  (Rendering|Components|Light|SetLightColor _sconcelight (Variables|Light|GetColor) true)
  (Rendering|Lighting|SetInnerConeAngle _sconcelight (Variables|Light|GetInner%20Cone%20Angle))
  (Rendering|Lighting|SetOuterConeAngle _sconcelight (Variables|Light|GetOuter%20Cone%20Angle))
  (LocalVariables|SetBarvaZarovicky "(R=1.000000,G=0.912440,B=0.850856,A=1.000000)")
  (Rendering|Components|Light|SetLightColor (Variables|Default|GetZarovicka) (LocalVariables|GetBarvaZarovicky) true))

(fn NastavRoznuti
  (params (ma%20svitit :type Boolean))
  (Variables|Moje|SetSvitime ma%20svitit)
  (Rendering|SetVisibility (Variables|Default|GetSconceLight) ma%20svitit false))

(fn Zruď
  (bind _sconcelight (Variables|Default|GetSconceLight))
  (Rendering|Components|Light|SetLightColor _sconcelight (Utilities|Struct|MakeLinearColor 1e+01 0.0 0.0 0.0) true)
  (Rendering|SetVisibility _sconcelight true false))