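; Player controller for the Skvt game that sets up Enhanced Input, the HUD, character swapping and the pause menu.
; BeginPlay adds the mapping contexts and creates the HUD, which binds to the controlled pawn's health component.
; The swap input possesses the next BP_SkvtBaseChar in the level, wrapping around, then rebinds the HUD.
; The menu input toggles the pausing main menu; helpers restart the level and show or close a text message widget.
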(event Input|EnhancedActionEvents|EnhancedInputActionIA_OpenMenu
  (params (ActionValue :type Boolean) (ElapsedSeconds :type Float%20%28double-precision%29) (TriggeredSeconds :type Float%20%28double-precision%29) (InputAction :type Input%20Action%20Object%20Reference :default "/Game/Skvt/UI/Input/IA_OpenMenu.IA_OpenMenu"))
  ;[0.05098 0.05098 0.05098] Prace s menu - klavesa P, Esc, namapováno v IMC_Default
  (bind _isotevrene (CallFunction|IsMenuOtevrene))
  (if _isotevrene
    (CallFunction|ZavriMenu (Variables|Default|GetMenuWidget))
    (else
      (CallFunction|OpenMenu))))

(event Input|EnhancedActionEvents|EnhancedInputActionIA_Swap
  (params (ActionValue :type Boolean) (ElapsedSeconds :type Float%20%28double-precision%29) (TriggeredSeconds :type Float%20%28double-precision%29) (InputAction :type Input%20Action%20Object%20Reference :default "/Game/Skvt/Characters/Input/Actions/IA_Swap.IA_Swap"))
  ;[0.05098 0.05098 0.05098] Přepni na další postavičku - klávesa N
  (bind (_index _vsechnypostavicky) (CallFunction|VratIndexAktualniPostavicky))
  (bind _output (CallFunction|NajdiDalsiho _index _vsechnypostavicky))
  (Pawn|Possess _output)
  (CallFunction|ReinicializujHUD))

(event EventBeginPlay
  (bind _self self)
  (bind _returnvalue (PlayerController|LocalPlayerSubsystems|GetEnhancedInputLocalPlayerSubsystem _self))
  (Utilities|IsValid _returnvalue
    (:Is%20Valid
      (Input|AddMappingContext _returnvalue "/Game/ThirdPerson/Input/IMC_Default.IMC_Default" 0 "(bIgnoreAllPressedKeysUntilRelease=True,bForceImmediately=False,bNotifyUserSettings=False)")
      (Input|AddMappingContext _returnvalue "/Game/Skvt/Characters/Input/IMC_SwapPawn.IMC_SwapPawn" 0 "(bIgnoreAllPressedKeysUntilRelease=True,bForceImmediately=False,bNotifyUserSettings=False)")
      (Input|AddMappingContext _returnvalue "/Game/Skvt/Characters/Input/IMC_Camera.IMC_Camera" 0 "(bIgnoreAllPressedKeysUntilRelease=True,bForceImmediately=False,bNotifyUserSettings=False)")
      (Input|AddMappingContext _returnvalue "/Game/Skvt/Characters/Input/IMC_FirstThird.IMC_FirstThird" 0 "(bIgnoreAllPressedKeysUntilRelease=True,bForceImmediately=False,bNotifyUserSettings=False)")
      ;[0.05098 0.05098 0.5] Inicializace mapování běhu a plížení
      (Input|AddMappingContext _returnvalue "/Game/Skvt/Characters/Input/IMC_ZacniBezet.IMC_ZacniBezet" 0 "(bIgnoreAllPressedKeysUntilRelease=True,bForceImmediately=False,bNotifyUserSettings=False)")
      (Input|AddMappingContext _returnvalue "/Game/Skvt/Characters/Input/IMC_ZmenPlizeni.IMC_ZmenPlizeni" 0 "(bIgnoreAllPressedKeysUntilRelease=True,bForceImmediately=False,bNotifyUserSettings=False)")
      (CallFunction|UdelejHUD))))

(fn ConstructionScript)

(fn OpenMenu
  (bind _self self)
  (bind _returnvalue (UserInterface|CreateWidget "/Game/Skvt/UI/Widgets/Menu/WBP_MainMenu.WBP_MainMenu_C" _self))
  (bind _output_get (Variables|Default|SetMenuWidget _returnvalue))
  (UserInterface|Viewport|AddtoViewport _output_get 0)
  (Input|SetInputModeGameandUI _self 0 "DoNotLock" true false)
  (Variables|Default|SetbShowMouseCursor true)
  (Game|SetGamePaused true))

(fn ZavriMenu
  (params (Menu :type WBP%20Main%20Menu%20Object%20Reference))
  (Default|ZavriMne Menu)
  (Game|SetGamePaused false))

(fn IsMenuOtevrene
  (return (Utilities|IsValid (Variables|Default|GetMenuWidget))))

(fn RestartujLevel
  (params (Menu :type WBP%20Main%20Menu%20Object%20Reference))
  (CallFunction|ZavriMenu Menu)
  (Game|OpenLevel(byObjectReference) "/Game/Skvt/SkvtProjectMap.SkvtProjectMap"))

(fn ZobrazZprvBdrchm
  (bind _self self)
  (bind _returnvalue (UserInterface|CreateWidget "/Game/Skvt/UI/Widgets/ZprvBdrchm/WBP_ZprvBdrchmTextWidget.WBP_ZprvBdrchmTextWidget_C" _self))
  (bind _output_get (Variables|Default|SetZprvBdrchmTextWidget _returnvalue))
  (UserInterface|Viewport|AddtoViewport _output_get 0)
  (Input|SetInputModeGameandUI _self 0 "DoNotLock" true false))

(fn ZavriZprvBdrchm
  (params (Widget :type WBP%20Zprv%20Bdrchm%20Text%20Widget%20Object%20Reference))
  (Default|ZavriMne Widget)
  (Game|SetGamePaused false))

(fn VratIndexAktualniPostavicky
  (bind _outactors (Actor|GetAllActorsOfClass "/Game/Skvt/Characters/BP_SkvtBaseChar.BP_SkvtBaseChar_C"))
  (bind _asbp_skvt_base_char (Utilities|Casting|CastToBP_SkvtBaseChar (Pawn|GetControlledPawn))
    (:then
      ;[1 1 1] Error handling
      (if (< (Utilities|Array|FindItem _outactors _asbp_skvt_base_char) 0)
        _
        (else
          (return (Utilities|Array|FindItem _outactors _asbp_skvt_base_char) _outactors))))
    (:CastFailed
      _))
  (Development|PrintString "Spatny pajdulak")
  (return -1 0))

(fn NajdiDalsiho
  (params (index :type Integer) (postavicky :type Array%20of%20BP%20Skvt%20Base%20Char%20Object%20References))
  (bind _result (Math|Integer|IncrementInt index)
    (:%20%20
      (return (Utilities|Array|Get(acopy) postavicky (Math|Integer|%(Integer) _result (Utilities|Array|Length postavicky)))))))

(fn UdelejHUD
  (bind _returnvalue (UserInterface|CreateWidget "/Game/Skvt/UI/Widgets/HUD/WBP_SkvtHUD.WBP_SkvtHUD_C" self))
  (bind _output_get (Variables|Default|SetMujHUD _returnvalue))
  (UserInterface|Viewport|AddtoViewport _output_get 0)
  (CallFunction|ReinicializujHUD))

(fn ReinicializujHUD
  (Default|InitMujHUD (Variables|Default|GetMujHUD) (Actor|GetComponentbyClass (Pawn|GetControlledPawn) "/Game/Skvt/Systems/DamageSystem/BP_SkvtHealtComponent.BP_SkvtHealtComponent_C")))