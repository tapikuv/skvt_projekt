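; Base NPC character with health, hit reactions, death, revival and player sighting.
; Damage goes to the health component with a punch montage; death plays a groin-kick montage, then a timer triggers ragdoll physics and disables movement.
; Revival refills health and replays both montages, without undoing the ragdoll.
; PawnSensing flags SeenPlayer on the AI blackboard and sets the player's, not the NPC's, walk speed.
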(event OnUmrel(BP_SkvtHealtComponent)
  (Animation|PlayAnimMontage "/Game/Skvt/Characters/Animations/Attacks/AM_Hit_GroinKick.AM_Hit_GroinKick" 1.0 "None")
  (Utilities|Time|SetTimerbyFunctionName 0 "SpustSmrt" 4.5))

(event OnObzivl(BP_SkvtHealtComponent)
  (bind _bp_skvthealtcomponent (Variables|Default|GetBP_SkvtHealtComponent))
  (Variables|/Game/Skvt/Systems/DamageSystem/BP_SkvtHealtComponent.BP_SkvtHealtComponent_C|SetZdravi _bp_skvthealtcomponent (Variables|/Game/Skvt/Systems/DamageSystem/BP_SkvtHealtComponent.BP_SkvtHealtComponent_C|GetZdraviMax _bp_skvthealtcomponent))
  (Animation|PlayAnimMontage "/Game/Skvt/Characters/Animations/Attacks/AM_Hit_punch.AM_Hit_punch" 1.0 "None")
  (Animation|PlayAnimMontage "/Game/Skvt/Characters/Animations/Attacks/AM_Hit_GroinKick.AM_Hit_GroinKick" 1.0 "None"))

(event OnSeePawn(PawnSensing)
  (params (Pawn :type Pawn%20Object%20Reference))
  (bind _returnvalue (Game|GetPlayerCharacter 0))
  (if (== Pawn _returnvalue)
    (AI|Components|Blackboard|SetValueasBool (AI|GetBlackboard (AI|GetAIController self)) (Utilities|Name|MakeLiteralName "SeenPlayer") true)
    (Variables|/Script/Engine.CharacterMovementComponent|SetMaxWalkSpeed (Variables|/Script/Engine.Character|GetCharacterMovement _returnvalue) 6e+02)))

(event EventBeginPlay)

(event Collision|EventActorBeginOverlap
  (params (OtherActor :type Actor%20Object%20Reference)))

(event EventTick
  (params (DeltaSeconds :type Float%20%28single-precision%29)))

(event Game|Damage|EventAnyDamage
  (params (Damage :type Float%20%28single-precision%29) (DamageType :type Damage%20Type%20Object%20Reference) (InstigatedBy :type Controller%20Object%20Reference) (DamageCauser :type Actor%20Object%20Reference))
  (Default|AplikujZraneni (Variables|Default|GetBP_SkvtHealtComponent) Damage)
  (Animation|PlayAnimMontage "/Game/Skvt/Characters/Animations/Attacks/AM_Hit_punch.AM_Hit_punch" 1.0 "None"))

(fn ConstructionScript)

(fn SpustSmrt
  (Physics|SetSimulatePhysics (Variables|Character|GetMesh) true)
  (Pawn|Components|CharacterMovement|DisableMovement (Variables|Character|GetCharacterMovement)))