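; BP_SkvtGameMode is the game mode that hands player control over to the next living character.
; BeginPlay caches the Skvt player controller.
; PossessNextCharakter calls NajdiDalsiPostavicku, which scans all BP_SkvtBaseChar actors for the first one not flagged JeMertvy.
; The controller then possesses that character via PosedniDalsiho, or opens the menu if none is found.
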(event Custom|PossessNextCharakter
  (bind _dalsipostavicka (CallFunction|NajdiDalsiPostavicku))
  (Utilities|IsValid _dalsipostavicka
    (:Is%20Valid
      (Default|PosedniDalsiho (Variables|Default|GetAs%20BP%20Skvt%20Player%20Controller) _dalsipostavicka))
    (:Is%20Not%20Valid
      (Default|OpenMenu (Variables|Default|GetAs%20BP%20Skvt%20Player%20Controller)))))

(event EventBeginPlay
  (bind _asbp_skvt_player_controller (Utilities|Casting|CastToBP_SkvtPlayerController (Game|GetPlayerController 0)))
  (Variables|Default|SetAs%20BP%20Skvt%20Player%20Controller _asbp_skvt_player_controller))

(fn ConstructionScript)

(fn NajdiDalsiPostavicku
  (bind _outactors (Actor|GetAllActorsOfClass "/Game/Skvt/Characters/BP_SkvtBaseChar.BP_SkvtBaseChar_C"))
  (if (Utilities|Array|IsNotEmpty _outactors)
    ;[1 1 1] Hledame prvního nemrtvého
    (for _array_element _outactors
      (if (not (Variables|/Game/Skvt/Characters/BP_SkvtBaseChar.BP_SkvtBaseChar_C|GetJeMertvy _array_element))
        (LocalVariables|SetNalezenaPostavicka _array_element)
        (return (LocalVariables|GetNalezenaPostavicka))))
    (return (LocalVariables|GetNalezenaPostavicka))))